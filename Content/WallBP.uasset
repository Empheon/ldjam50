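; Grid-based wall actor that picks its mesh and rotation to connect with neighbouring walls.
; On BeginPlay, RefreshWall line-traces one grid step in four directions to store adjacent WallBP actors.
; The neighbour count, plus a straight-versus-corner check, selects the static mesh, and neighbour layout sets its yaw.
; It then refreshes each neighbour without further propagation, so existing walls adapt to a new one.
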(event `self.ReceiveBeginPlay`
  (`self.RefreshWall` true))

(fn `GetAdjacentWall`
  (params (XOffset :type "Float (double-precision)") (YOffset :type "Float (double-precision)"))
  (returns (Wall :type "/Game/WallBP Object Reference"))
  (bind (_returnvalue_x _returnvalue_y) (`KismetMathLibrary.BreakVector` (`self.K2_GetActorLocation`)))
  (bind (_outhit _returnvalue) (`KismetSystemLibrary.LineTraceSingleForObjects` (`KismetMathLibrary.MakeVector` _returnvalue_x _returnvalue_y 10.0) (`KismetMathLibrary.MakeVector` (+ _returnvalue_x XOffset) (+ _returnvalue_y YOffset) 10.0) (`|MakeArray` "ObjectTypeQuery9" :!type "EObjectTypeQuery Enum")))
  (if _returnvalue
    (bind _aswall_bp (cast `/Game/WallBP` (`.HitActor` (`GameplayStatics.BreakHitResult` _outhit)))
      (:`then`
        (return _aswall_bp))
      (:`CastFailed`
        (return null)))))

(fn `RefreshWall`
  (params (RefreshAdjacents :type Boolean))
  (locals (TopWall :type "/Game/WallBP Object Reference") (BottomWall :type "/Game/WallBP Object Reference") (RightWall :type "/Game/WallBP Object Reference") (LeftWall :type "/Game/WallBP Object Reference") (AdjacentCount :type Integer) (MeshId :type Integer))
  (bind _topwall (`local.TopWall`))
  (bind _bottomwall (`local.BottomWall`))
  (bind _rightwall (`local.RightWall`))
  (bind _leftwall (`local.LeftWall`))
  (bind _returnvalue (select `bool` (== (`local.AdjacentCount`) 2) :`false` (`local.AdjacentCount`) :`true` (select `bool` (or (and (`KismetSystemLibrary.IsValid` (`local.TopWall`)) (`KismetSystemLibrary.IsValid` (`local.BottomWall`))) (and (`KismetSystemLibrary.IsValid` (`local.RightWall`)) (`KismetSystemLibrary.IsValid` (`local.LeftWall`)))) :`false` 2 :`true` 1)))
  (`|ExecutionSequence`
    (:`then_0`
      (bind _wall (`self.GetAdjacentWall` 200.0))
      (set `local.TopWall` _wall)
      (bind _wall_2 (`self.GetAdjacentWall` -200.0))
      (set `local.BottomWall` _wall_2)
      (bind _wall_3 (`self.GetAdjacentWall` 0.0 200.0))
      (set `local.RightWall` _wall_3)
      (bind _wall_4 (`self.GetAdjacentWall` 0.0 -200.0))
      (set `local.LeftWall` _wall_4))
    (:`then_1`
      (`/Engine/EditorBlueprintResources/StandardMacros.IsValid` (`local.TopWall`)
        (:`Is Valid`
          (`/Engine/EditorBlueprintResources/StandardMacros.IncrementInt` (`local.AdjacentCount`)
            (:`  `
              _)))
        (:`Is Not Valid`
          _))
      (`/Engine/EditorBlueprintResources/StandardMacros.IsValid` (`local.BottomWall`)
        (:`Is Valid`
          (`/Engine/EditorBlueprintResources/StandardMacros.IncrementInt` (`local.AdjacentCount`)
            (:`  `
              _)))
        (:`Is Not Valid`
          _))
      (`/Engine/EditorBlueprintResources/StandardMacros.IsValid` (`local.RightWall`)
        (:`Is Valid`
          (`/Engine/EditorBlueprintResources/StandardMacros.IncrementInt` (`local.AdjacentCount`)
            (:`  `
              _)))
        (:`Is Not Valid`
          _))
      (`/Engine/EditorBlueprintResources/StandardMacros.IsValid` (`local.LeftWall`)
        (:`Is Valid`
          (`/Engine/EditorBlueprintResources/StandardMacros.IncrementInt` (`local.AdjacentCount`)))))
    (:`then_2`
      ;[1 1 1] Update Mesh
      (set `local.MeshId` _returnvalue)
      (`StaticMeshComponent.SetStaticMesh` (`self.Cube`) (select `int` _returnvalue :`0` "/Game/Resources/Buildings/Buildings_Wall_All_Side.Buildings_Wall_All_Side" :`1` "/Game/Resources/Buildings/Buildings_Wall_Two_Side.Buildings_Wall_Two_Side" :`2` "/Game/Resources/Buildings/Buildings_Wall_Corner.Buildings_Wall_Corner" :`3` "/Game/Resources/Buildings/Buildings_Wall_One_Side.Buildings_Wall_One_Side" :`4` "/Game/Resources/Buildings/Buildings_Wall_All.Buildings_Wall_All" :!type "StaticMesh Object Reference")))
    (:`then_3`
      (`|ExecutionSequence`
        (:`then_0`
          ;[1 1 1] Side Walls
          (if (== (`local.MeshId`) 1)
            (if (!= (`local.AdjacentCount`) 1)
              (`SceneComponent.K2_SetWorldRotation` (`self.Cube`) (select `bool` (and (`KismetSystemLibrary.IsValid` (`local.TopWall`)) (`KismetSystemLibrary.IsValid` (`local.BottomWall`))) :`true` (struct :`Yaw` 90.0) :!type "Rotator Structure") false false)
              (else
                (`SceneComponent.K2_SetWorldRotation` (`self.Cube`) (select `bool` (or (`KismetSystemLibrary.IsValid` (`local.TopWall`)) (`KismetSystemLibrary.IsValid` (`local.BottomWall`))) :`true` (struct :`Yaw` 90.0) :!type "Rotator Structure") false false)))))
        (:`then_1`
          ;[1 1 1] Corners
          (if (== (`local.MeshId`) 2)
            (`/Engine/EditorBlueprintResources/StandardMacros.IsValid` (`local.TopWall`)
              (:`Is Valid`
                (`/Engine/EditorBlueprintResources/StandardMacros.IsValid` (`local.RightWall`)
                  (:`Is Valid`
                    (`SceneComponent.K2_SetWorldRotation` (`self.Cube`) (struct :`Yaw` 270.0) false false))
                  (:`Is Not Valid`
                    (`SceneComponent.K2_SetWorldRotation` (`self.Cube`) (struct :`Yaw` 180.0) false false))))
              (:`Is Not Valid`
                (`/Engine/EditorBlueprintResources/StandardMacros.IsValid` (`local.RightWall`)
                  (:`Is Valid`
                    (`SceneComponent.K2_SetWorldRotation` :`self` (`self.Cube`)))
                  (:`Is Not Valid`
                    (`SceneComponent.K2_SetWorldRotation` (`self.Cube`) (struct :`Yaw` 90.0) false false)))))))
        (:`then_2`
          ;[1 1 1] T Shape
          (if (== (`local.MeshId`) 3)
            (`/Engine/EditorBlueprintResources/StandardMacros.IsValid` (`local.TopWall`)
              (:`Is Valid`
                (`/Engine/EditorBlueprintResources/StandardMacros.IsValid` (`local.BottomWall`)
                  (:`Is Valid`
                    (`/Engine/EditorBlueprintResources/StandardMacros.IsValid` (`local.RightWall`)
                      (:`Is Valid`
                        (`/Engine/EditorBlueprintResources/StandardMacros.IsValid` (`local.LeftWall`)
                          (:`Is Not Valid`
                            (`SceneComponent.K2_SetWorldRotation` (`self.Cube`) (struct :`Yaw` 270.0) false false))))
                      (:`Is Not Valid`
                        (`SceneComponent.K2_SetWorldRotation` (`self.Cube`) (struct :`Yaw` 90.0) false false))))
                  (:`Is Not Valid`
                    (`SceneComponent.K2_SetWorldRotation` (`self.Cube`) (struct :`Yaw` 180.0) false false))))
              (:`Is Not Valid`
                (`SceneComponent.K2_SetWorldRotation` :`self` (`self.Cube`))))))))
    (:`then_4`
      (if RefreshAdjacents
        (`/Engine/EditorBlueprintResources/StandardMacros.IsValid` _topwall
          (:`Is Valid`
            (`self.RefreshWall` _topwall false))
          (:`Is Not Valid`
            _))
        (`/Engine/EditorBlueprintResources/StandardMacros.IsValid` _bottomwall
          (:`Is Valid`
            (`self.RefreshWall` _bottomwall false))
          (:`Is Not Valid`
            _))
        (`/Engine/EditorBlueprintResources/StandardMacros.IsValid` _rightwall
          (:`Is Valid`
            (`self.RefreshWall` _rightwall false))
          (:`Is Not Valid`
            _))
        (`/Engine/EditorBlueprintResources/StandardMacros.IsValid` _leftwall
          (:`Is Valid`
            (`self.RefreshWall` _leftwall false)))))))

(fn `UserConstructionScript`)