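; Archer tower Blueprint that turns its Weapon component to face the direction it shoots.
; The OnShoot event flattens the shot direction to the horizontal plane and stores it as a target rotation.
; Tick eases the weapon's world rotation toward that target with a shortest-path lerp scaled by delta time.
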(event `self.ReceiveTick`
  (params (DeltaSeconds :type "Float (single-precision)"))
  (bind _weapon (`self.Weapon`))
  (`SceneComponent.K2_SetWorldRotation` _weapon (`KismetMathLibrary.RLerp` (`SceneComponent.K2_GetComponentRotation` _weapon) (`self.TargetRotation`) (* DeltaSeconds 10.0) true) false false))

(event `self.OnShoot`
  (params (direction :type "Vector Structure"))
  (set `self.TargetRotation` (`KismetMathLibrary.MakeRotFromX` (`KismetMathLibrary.Normal` (`KismetMathLibrary.MakeVector` (.x direction) (.y direction))))))

(fn `UserConstructionScript`)